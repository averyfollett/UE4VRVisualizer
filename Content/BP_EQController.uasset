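; BP_EQController is an audio visualizer that turns a grid of spawned BP_Cube actors into an animated equalizer for a music track.
; On BeginPlay it starts audio and spawns cubes in rows, columns and levels, rotated and offset by its own transform.
; Each Tick it samples the track's frequency spectrum at current game time, one band per cube, setting that cube's world Z and blended color from the magnitude.
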(event `self.ReceiveBeginPlay`
  (`AudioComponent.Play` (`self.Audio`) 0.0)
  (`self.SpawnGrid`))

(event `self.ReceiveTick`
  (params (DeltaSeconds :type "Float (single-precision)"))
  (bind _outspectrum (`SoundVisualizationStatics.CalculateFrequencySpectrum` (`self.Track`) 0 (`KismetSystemLibrary.GetGameTimeInSeconds`) 0.1 (`KismetArrayLibrary.Array_Length` (`self.BP_CubeArray`))))
  (set `self.Spectrum` _outspectrum)
  (for (_array_element _array_index) (`self.BP_CubeArray`)
    (bind (_returnvalue_x _returnvalue_y) (`KismetMathLibrary.BreakVector` (`self.K2_GetActorLocation` _array_element)))
    (bind _returnvalue (`KismetMathLibrary.Abs` (`|GetArrayItem` (`self.Spectrum`) _array_index)))
    (`self.K2_SetActorTransform` _array_element (`KismetMathLibrary.MakeTransform` (`KismetMathLibrary.MakeVector` _returnvalue_x _returnvalue_y (* _returnvalue 10.0))) false false)
    (set `/Game/BP_Cube.CurrentColor` (`KismetMathLibrary.LinearColorLerp` (`self.LerpColor1`) (`self.LerpColor2`) (/ _returnvalue 20.0)) _array_element)))

(fn `SpawnGrid`
  (bind _row (`self.Row`))
  (for _ (range (`self.NumCubes`))
    (bind _returnvalue (`|SpawnActorFromClass` "/Game/BP_Cube.BP_Cube_C" (`KismetMathLibrary.MakeTransform` (+ (`KismetMathLibrary.GreaterGreater_VectorRotator` (`KismetMathLibrary.MakeVector` (* (`self.Row`) (`self.Distance`)) (* (`self.Column`) (`self.Distance`)) (* (`self.Level`) (`self.Distance`))) (`self.K2_GetActorRotation`)) (`self.K2_GetActorLocation`))) "AlwaysSpawn" "OverrideRootScale" null null))
    (`KismetArrayLibrary.Array_Add` (`self.BP_CubeArray`) _returnvalue)
    (`/Engine/EditorBlueprintResources/StandardMacros.IncrementInt` _row
      (:`  `
        (if (== _row (`self.NumRows`))
          (bind _result (`/Engine/EditorBlueprintResources/StandardMacros.IncrementInt` (`self.Column`))
            (:`  `
              (set `self.Row` 0)
              (if (== _result (`self.NumColumns`))
                (`/Engine/EditorBlueprintResources/StandardMacros.IncrementInt` (`self.Level`)
                  (:`  `
                    (set `self.Row` 0)
                    (set `self.Column` 0)))))))))))

(fn `UserConstructionScript`)